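; TrumpFloatingHead is a floating head actor with left and right face components under their own materials and an animated Head component.
; Its construction script assigns each face material and sets the matching left or right opacity parameter to fully opaque.
; On BeginPlay, the MovementScale timeline drives the Head's roll and uniform scale each update, holding its relative location at the origin.
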(event EventBeginPlay
  (bind (_direction _scale _rotation) (Timeline|Movement&Scale PlayFromStart)
    (:Update
      (Transformation|SetRelativeTransform (Variables|Default|GetHead) (Math|Transform|MakeTransform "0, 0, 0" (Math|Rotator|MakeRotator _rotation 0.0 0.0) (Math|Conversions|ToVector(Float) _scale)) false false))))

(fn ConstructionScript
  (bind _left_face (Variables|Default|Getleft_face))
  (bind _right_face (Variables|Default|Getright_face))
  (Rendering|Material|SetMaterial _left_face 0 (Variables|Default|GetLeftFaceMat))
  (Rendering|Material|SetMaterial _right_face 0 (Variables|Default|GetRightFaceMat))
  (Rendering|Material|SetScalarParameterValueonMaterials _left_face "LeftOpacity" 1.0)
  (Rendering|Material|SetScalarParameterValueonMaterials _right_face "RightOpacity" 1.0))