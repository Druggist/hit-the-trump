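; Trump is a hittable head actor that the player's FirstPersonCharacter strikes on its left or right side until it wins the level.
; Each hit plays a timeline that rotates the Head, then raises that side's material opacity parameter.
; If the character is flagged special, a SpecialAttack timeline pitches the Head and raises both sides at once.
; When both opacities reach full, Win opens InitialMap.
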(event Collision|EventHit
  (params (MyComp :type Primitive%20Component%20Object%20Reference) (Other :type Actor%20Object%20Reference) (OtherComp :type Primitive%20Component%20Object%20Reference) (bSelfMoved :type Boolean) (HitLocation :type Vector :default "0, 0, 0") (HitNormal :type Vector :default "0, 0, 0") (NormalImpulse :type Vector :default "0, 0, 0") (Hit :type Hit%20Result%20Structure%20%28by%20ref%29))
  (bind _asfirst_person_character (Utilities|Casting|CastToFirstPersonCharacter Other))
  (if (Variables|/Game/Blueprints/FirstPersonCharacter.FirstPersonCharacter_C|GetisSpecial _asfirst_person_character)
    (Variables|Default|SetIsSpecial true))
  (if (== MyComp (Variables|Default|GetrightH))
    (if (Variables|Default|GetIsSpecial)
      (bind _lefthit (Timeline|SpecialAttack PlayFromStart)
        (:Update
          (Transformation|SetWorldRotation (Variables|Default|Gethead) (Math|Rotator|MakeRotator 0.0 (* _lefthit 1e+02) 0.0) false false))
        (:Finished
          (CallFunction|AddRightOpacity)
          (CallFunction|AddLeftOpacity)
          (Variables|Default|SetIsSpecial false :!label _label)
          (if (and (>= (Variables|Default|GetLeftOpacity) 1.0) (>= (Variables|Default|GetRightOpacity) 1.0))
            (CallFunction|Win))))
      (else
        (bind _lefthit_2 (Timeline|RightHit PlayFromStart)
          (:Update
            (Transformation|SetWorldRotation (Variables|Default|Gethead) (Math|Rotator|MakeRotator (* _lefthit_2 1e+02) 0.0 0.0) false false))
          (:Finished
            (CallFunction|AddRightOpacity)
            (goto _label)))))
    (elif (== MyComp (Variables|Default|GetleftH))
      (if (Variables|Default|GetIsSpecial)
        (Timeline|SpecialAttack PlayFromStart)
        (else
          (bind _lefthit_3 (Timeline|LeftHit PlayFromStart)
            (:Update
              (Transformation|SetWorldRotation (Variables|Default|Gethead) (Math|Rotator|MakeRotator (* _lefthit_3 1e+02) 0.0 0.0) false false))
            (:Finished
              (CallFunction|AddLeftOpacity)
              (goto _label))))))))

(fn ConstructionScript)

(fn AddRightOpacity
  (bind _output_get (Variables|Default|SetRightOpacity (+ (Variables|Default|GetOpacityMultipler) (Variables|Default|GetRightOpacity))))
  (Rendering|Material|SetScalarParameterValueonMaterials (Variables|Default|GetrightH) "RightOpacity" _output_get)
  (return))

(fn AddLeftOpacity
  (bind _output_get (Variables|Default|SetLeftOpacity (+ (Variables|Default|GetOpacityMultipler) (Variables|Default|GetLeftOpacity))))
  (Rendering|Material|SetScalarParameterValueonMaterials (Variables|Default|GetleftH) "LeftOpacity" _output_get)
  (return))

(fn Win
  (Game|OpenLevel(byName) "InitialMap")
  (return))